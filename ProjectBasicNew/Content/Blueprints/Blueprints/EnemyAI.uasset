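; EnemyAI is an enemy character that takes gun-dependent damage, respawns on death and awards the player points.
; BeginPlay spawns its default controller, then sets the AI controller class and full health.
; Any hit on its Sphere component subtracts health according to the FirstPersonCharacter's current gun, without checking what struck it.
; At zero health it spawns a replacement at the first Spawn1 actor, destroys itself and increments the player's Points.
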(event OnComponentHit(Sphere)
  (params (HitComponent :type Primitive%20Component%20Object%20Reference) (OtherActor :type Actor%20Object%20Reference) (OtherComp :type Primitive%20Component%20Object%20Reference) (NormalImpulse :type Vector :default "0, 0, 0") (Hit :type Hit%20Result%20Structure%20%28by%20ref%29))
  ;[1 1 1] AI character when hit by the balls it detects which gun the fps player is holding and decrease their health according to that gun and dies when the health reaches 0
  (Utilities|FlowControl|Sequence ; Execute the blocks of code in proper order
    (:then_0
      (bind _returnvalue (Actor|GetActorOfClass "/Game/Blueprints/Blueprints/FirstPersonCharacter.FirstPersonCharacter_C"))
      (if (== (Variables|/Game/Blueprints/Blueprints/FirstPersonCharacter.FirstPersonCharacter_C|GetGuns _returnvalue) 0)
        (Variables|Default|SetHealth (- (Variables|Default|GetHealth) 50))
        (elif (== (Variables|/Game/Blueprints/Blueprints/FirstPersonCharacter.FirstPersonCharacter_C|GetGuns _returnvalue) 1)
          (Variables|Default|SetHealth (- (Variables|Default|GetHealth) 35))
          (elif (== (Variables|/Game/Blueprints/Blueprints/FirstPersonCharacter.FirstPersonCharacter_C|GetGuns _returnvalue) 2)
            (Variables|Default|SetHealth (- (Variables|Default|GetHealth) 35))))))
    (:then_1
      (if (<= (Variables|Default|GetHealth) 0)
        (Variables|Default|SetDead true)
        (bind _outactors (Actor|GetAllActorsOfClass "/Game/Blueprints/Blueprints/spawn1.spawn1_C"))
        (Game|SpawnActorfromClass "EnemyAI_C" (Transformation|GetActorTransform (Utilities|Array|Get(acopy) _outactors)) "AdjustIfPossibleButAlwaysSpawn" 0 0)
        (Actor|DestroyActor)
        ;[1 1 1] Point system(getting the points from the FPS character and increasing it)
        (bind _returnvalue_2 (Actor|GetActorOfClass "/Game/Blueprints/Blueprints/FirstPersonCharacter.FirstPersonCharacter_C"))
        (bind _output_get (Variables|Default|SetFPS%20character%20ref _returnvalue_2))
        (Variables|/Game/Blueprints/Blueprints/FirstPersonCharacter.FirstPersonCharacter_C|SetPoints _output_get (+ (Variables|/Game/Blueprints/Blueprints/FirstPersonCharacter.FirstPersonCharacter_C|GetPoints _output_get) 1))))))

(event EventTick
  (params (DeltaSeconds :type Float%20%28single-precision%29)))

(event EventBeginPlay
  ;[1 1 1] Spawns the AI controller class when the AI spawned
  (Pawn|SpawnDefaultController)
  (Variables|Default|SetAIControllerClass "/Game/Blueprints/Blueprints/AI.AI_C")
  (Variables|Default|SetHealth 100)
  (Variables|Default|SetDead false))

(fn ConstructionScript)